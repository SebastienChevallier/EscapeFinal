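; BP_Trapdoor is a trapdoor that tracks an open/closed state and plays sounds for opening, closing and being stepped on.
; ToggleState flips the state, GetState reports it, and OnRotationChanged moves the scene's yaw into pitch.
; PlaySound plays locker sounds scaled by GameInstance SFX volume, delaying the close.
; First-person character overlaps, except its pick zone, trigger an unscaled floor squeak, throttled by a timed flag.
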(event `/Game/Blueprints/Interfaces/BPI_Interaction.ToggleState`
  (set `self.IsOpen` (not (`self.IsOpen`))))

(event `/Game/Blueprints/Interfaces/BPI_Interaction.OnRotationChanged`
  (bind _scene (`self.Scene`))
  (bind (_relativerotation_roll _relativerotation_pitch _relativerotation_yaw) (`KismetMathLibrary.BreakRotator` (`SceneComponent.RelativeRotation` _scene)))
  (`SceneComponent.K2_SetRelativeRotation` _scene (`KismetMathLibrary.MakeRotator` 0.0 _relativerotation_yaw) false false))

(event `/Game/Blueprints/Interfaces/BPI_Interaction.PlaySound`
  (params (Action :type String) (Actor :type "Actor Object Reference"))
  (bind _returnvalue (`self.K2_GetActorLocation` Actor))
  (bind _asbp_game_instance (cast `/Game/FirstPerson/Blueprints/BP_GameInstance` (`GameplayStatics.GetGameInstance`)))
  (bind _sfxvolume (`/Game/FirstPerson/Blueprints/BP_GameInstance.GetSfxVolume` _asbp_game_instance))
  (switch `string` Action
    (:`Open`
      (bind _returnvalue_2 (* _sfxvolume 2.0))
      (`GameplayStatics.PlaySoundAtLocation` "/Game/Audio/Sounds/LockerOpening.LockerOpening" _returnvalue (struct) _returnvalue_2 1.0 0.0 null null null null))
    (:`Close`
      (`KismetSystemLibrary.Delay` 0.8)
      (`GameplayStatics.PlaySoundAtLocation` "/Game/Audio/Sounds/LockerClosing.LockerClosing" _returnvalue (struct) _returnvalue_2 1.0 0.0 null null null null))))

(event `self.Trigger.OnComponentBeginOverlap`
  (params (OverlappedComponent :type "PrimitiveComponent Object Reference") (OtherActor :type "Actor Object Reference") (OtherComp :type "PrimitiveComponent Object Reference") (OtherBodyIndex :type Integer) (bFromSweep :type Boolean) (SweepResult :type "HitResult Structure (by ref)"))
  (bind _asbp_first_person_character (cast `/Game/FirstPerson/Blueprints/BP_FirstPersonCharacter` OtherActor))
  (if (== OtherComp (`/Game/FirstPerson/Blueprints/BP_FirstPersonCharacter.CanPickZone` _asbp_first_person_character))
    _
    (elif (not (`self.IsPlayingSound`))
      (`GameplayStatics.PlaySoundAtLocation` "/Game/Audio/Sounds/Squeaking_floor.Squeaking_floor" (`self.K2_GetActorLocation`) (struct) 0.2 1.0 0.0 null null null null)
      (set `self.IsPlayingSound` true)
      (`KismetSystemLibrary.Delay` 2.88)
      (set `self.IsPlayingSound` false))))

(fn `Get State`
  (returns (isOpen :type Boolean))
  (return (`self.IsOpen`)))

(fn `UserConstructionScript`)