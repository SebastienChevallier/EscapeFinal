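; BP_Carpet is a carpet actor with toggle and state functions, where rotation input becomes a sideways slide.
; On a rotation change, it sets the Scene component's relative X location from its yaw, scaled and negated, then zeroes the rotation.
; ToggleState only clears the actor's tags, while GetState returns IsOpen, which these graphs never set.
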(event `/Game/Blueprints/Interfaces/BPI_Interaction.ToggleState`
  (`KismetArrayLibrary.Array_Clear` (`self.Tags`)))

(event `/Game/Blueprints/Interfaces/BPI_Interaction.OnRotationChanged`
  (bind (_relativerotation_roll _relativerotation_pitch _relativerotation_yaw) (`KismetMathLibrary.BreakRotator` (`SceneComponent.RelativeRotation` (`self.Scene`))))
  (`SceneComponent.K2_SetRelativeLocation` (`self.Scene`) (`KismetMathLibrary.MakeVector` (* _relativerotation_yaw -2.0) 0.0 0.0) false false)
  (`SceneComponent.K2_SetRelativeRotation` :`self` (`self.Scene`)))

(fn `Get State`
  (returns (isOpen :type Boolean))
  (return (`self.IsOpen`)))

(fn `UserConstructionScript`)