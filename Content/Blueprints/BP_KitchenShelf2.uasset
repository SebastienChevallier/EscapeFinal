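; BP_KitchenShelf2 is an openable kitchen shelf that tracks an open/closed state and plays cupboard sounds.
; ToggleState flips IsOpen, which GetState exposes to other objects.
; OnRotationChanged negates the Scene component's yaw.
; PlaySound plays open or delayed close audio at the given actor's location, scaled by the SFX volume from BP_GameInstance.
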(event `/Game/Blueprints/Interfaces/BPI_Interaction.OnRotationChanged`
  (bind _scene (`self.Scene`))
  (bind (_relativerotation_roll _relativerotation_pitch _relativerotation_yaw) (`KismetMathLibrary.BreakRotator` (`SceneComponent.RelativeRotation` _scene)))
  (`SceneComponent.K2_SetRelativeRotation` _scene (`KismetMathLibrary.MakeRotator` 0.0 0.0 (* _relativerotation_yaw -1.0)) false false))

(event `/Game/Blueprints/Interfaces/BPI_Interaction.ToggleState`
  (set `self.IsOpen` (not (`self.IsOpen`))))

(event `/Game/Blueprints/Interfaces/BPI_Interaction.PlaySound`
  (params (Action :type String) (Actor :type "Actor Object Reference"))
  (bind _returnvalue (`self.K2_GetActorLocation` Actor))
  (bind _asbp_game_instance (cast `/Game/FirstPerson/Blueprints/BP_GameInstance` (`GameplayStatics.GetGameInstance`)))
  (bind _sfxvolume (`/Game/FirstPerson/Blueprints/BP_GameInstance.GetSfxVolume` _asbp_game_instance))
  (switch `string` Action
    (:`Open`
      (`GameplayStatics.PlaySoundAtLocation` "/Game/Audio/Sounds/CupboardOpening.CupboardOpening" _returnvalue (struct) _sfxvolume 1.0 0.0 null null null null))
    (:`Close`
      (`KismetSystemLibrary.Delay` 0.7)
      (`GameplayStatics.PlaySoundAtLocation` "/Game/Audio/Sounds/DeskClosing.DeskClosing" _returnvalue (struct) _sfxvolume 1.0 0.0 null null null null))))

(fn `Get State`
  (returns (isOpen :type Boolean))
  (return (`self.IsOpen`)))

(fn `UserConstructionScript`)