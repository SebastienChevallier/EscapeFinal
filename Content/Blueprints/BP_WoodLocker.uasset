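; Wooden locker Blueprint that tracks whether it is open or closed.
; ToggleState flips the IsOpen flag and GetState returns it, with no movement or animation attached to either.
; A separate OnRotationChanged event mirrors the Scene component by negating its relative yaw and zeroing pitch and roll, independently of IsOpen.
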(event `/Game/Blueprints/Interfaces/BPI_Interaction.ToggleState`
  (set `self.IsOpen` (not (`self.IsOpen`))))

(event `/Game/Blueprints/Interfaces/BPI_Interaction.OnRotationChanged`
  (bind _scene (`self.Scene`))
  (bind (_relativerotation_roll _relativerotation_pitch _relativerotation_yaw) (`KismetMathLibrary.BreakRotator` (`SceneComponent.RelativeRotation` _scene)))
  (`SceneComponent.K2_SetRelativeRotation` _scene (`KismetMathLibrary.MakeRotator` 0.0 0.0 (* _relativerotation_yaw -1.0)) false false))

(fn `Get State`
  (returns (isOpen :type Boolean))
  (return (`self.IsOpen`)))

(fn `UserConstructionScript`)