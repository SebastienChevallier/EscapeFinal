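; BP_Door is a door actor that exposes an open-state query and handles toggle, rotation and sound events.
; ToggleState only clears the actor's tags, and GetState returns IsOpen, which no graph here sets.
; OnRotationChanged zeroes the Scene component's roll and pitch, keeping only yaw.
; PlaySound plays a cupboard-opening sound at the passed actor's location, scaled by the SFX volume from BP_GameInstance.
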(event `self.ToggleState`
  (`KismetArrayLibrary.Array_Clear` (`self.Tags`)))

(event `self.OnRotationChanged`
  (bind _scene (`self.Scene`))
  (bind (_relativerotation_roll _relativerotation_pitch _relativerotation_yaw) (`KismetMathLibrary.BreakRotator` (`SceneComponent.RelativeRotation` _scene)))
  (`SceneComponent.K2_SetRelativeRotation` _scene (`KismetMathLibrary.MakeRotator` 0.0 0.0 _relativerotation_yaw) false false))

(event `self.PlaySound`
  (params (Action :type String) (Actor :type "Actor Object Reference"))
  (bind _asbp_game_instance (cast `/Game/FirstPerson/Blueprints/BP_GameInstance` (`GameplayStatics.GetGameInstance`)))
  (bind _sfxvolume (`/Game/FirstPerson/Blueprints/BP_GameInstance.GetSfxVolume` _asbp_game_instance))
  (`GameplayStatics.PlaySoundAtLocation` "/Game/Audio/Sounds/CupboardOpening.CupboardOpening" (`self.K2_GetActorLocation` Actor) (struct) _sfxvolume 1.0 0.0 null null null null))

(fn `Get State`
  (returns (isOpen :type Boolean))
  (return (`self.IsOpen`)))

(fn `UserConstructionScript`)