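; BP_DoorLocks is a door lock actor with four locks that slide open one at a time.
; Each UnlockDoorLock call plays a sliding sound at the actor and starts a timeline that drives the relative X position of the lock selected by LockToUnlockIndex.
; When the timeline finishes, it increments the index, so the next call moves the following lock.
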(event `UnlockDoorLock`
  (bind (_relativelocation_x _relativelocation_y _relativelocation_z) (`KismetMathLibrary.BreakVector` (`SceneComponent.RelativeLocation` (`self.Lock4`))))
  (bind (_relativelocation_x_2 _relativelocation_y_2 _relativelocation_z_2) (`KismetMathLibrary.BreakVector` (`SceneComponent.RelativeLocation` (`self.Lock1`))))
  (bind (_relativelocation_x_3 _relativelocation_y_3 _relativelocation_z_3) (`KismetMathLibrary.BreakVector` (`SceneComponent.RelativeLocation` (`self.Lock2`))))
  (bind (_relativelocation_x_4 _relativelocation_y_4 _relativelocation_z_4) (`KismetMathLibrary.BreakVector` (`SceneComponent.RelativeLocation` (`self.Lock3`))))
  (`GameplayStatics.PlaySoundAtLocation` "/Game/Audio/Sounds/SlidingLibrary.SlidingLibrary" (`self.K2_GetActorLocation`) (struct) 1.0 1.0 0.0 null null null null)
  (bind (_direction _slidingvalue) (`Timeline|Timeline` :!via `PlayFromStart`)
    (:`Update`
      (switch `int` (`self.LockToUnlockIndex`)
        (:`1`
          (`SceneComponent.K2_SetRelativeLocation` (`self.Lock1`) (`KismetMathLibrary.MakeVector` _slidingvalue _relativelocation_y_2 _relativelocation_z_2) false false))
        (:`2`
          (`SceneComponent.K2_SetRelativeLocation` (`self.Lock2`) (`KismetMathLibrary.MakeVector` _slidingvalue _relativelocation_y_3 _relativelocation_z_3) false false))
        (:`3`
          (`SceneComponent.K2_SetRelativeLocation` (`self.Lock3`) (`KismetMathLibrary.MakeVector` _slidingvalue _relativelocation_y_4 _relativelocation_z_4) false false))
        (:`4`
          (`SceneComponent.K2_SetRelativeLocation` (`self.Lock4`) (`KismetMathLibrary.MakeVector` _slidingvalue _relativelocation_y _relativelocation_z) false false))))
    (:`Finished`
      (`/Engine/EditorBlueprintResources/StandardMacros.IncrementInt` (`self.LockToUnlockIndex`)))))

(fn `UserConstructionScript`)