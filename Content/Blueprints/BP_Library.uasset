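; Library actor that plays a squeaking floor sound when the first-person character enters its Trigger volume.
; Overlaps from the character's CanPickZone component are ignored.
; The sound plays at the actor's location, with a flag and a delay of just under three seconds blocking replays.
; GetState is a fixed stub that always returns false.
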(event `self.Trigger.OnComponentBeginOverlap`
  (params (OverlappedComponent :type "PrimitiveComponent Object Reference") (OtherActor :type "Actor Object Reference") (OtherComp :type "PrimitiveComponent Object Reference") (OtherBodyIndex :type Integer) (bFromSweep :type Boolean) (SweepResult :type "HitResult Structure (by ref)"))
  (bind _asbp_first_person_character (cast `/Game/FirstPerson/Blueprints/BP_FirstPersonCharacter` OtherActor))
  (if (== OtherComp (`/Game/FirstPerson/Blueprints/BP_FirstPersonCharacter.CanPickZone` _asbp_first_person_character))
    _
    (elif (not (`self.isPlayingSound`))
      (`GameplayStatics.PlaySoundAtLocation` "/Game/Audio/Sounds/Squeaking_floor.Squeaking_floor" (`self.K2_GetActorLocation`) (struct) 0.2 1.0 0.0 null null null null)
      (set `self.isPlayingSound` true)
      (`KismetSystemLibrary.Delay` 2.88)
      (set `self.isPlayingSound` false))))

(fn `Get State`
  (returns (isOpen :type Boolean))
  (return false))

(fn `UserConstructionScript`)