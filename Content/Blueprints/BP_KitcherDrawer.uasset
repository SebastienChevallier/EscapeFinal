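; Kitchen drawer Blueprint that tracks an open/closed state, slides, and plays opening and closing sounds.
; ToggleState flips IsOpen, which GetState reports.
; OnRotationChanged turns the Scene component's yaw into a Y-axis slide, then zeroes the rotation, so rotation input produces linear motion.
; PlaySound plays at the given actor's location, scaled by the GameInstance SFX volume, with a short delay before the closing sound.
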(event `/Game/Blueprints/Interfaces/BPI_Interaction.ToggleState`
  (set `self.IsOpen` (not (`self.IsOpen`))))

(event `/Game/Blueprints/Interfaces/BPI_Interaction.OnRotationChanged`
  (bind (_relativerotation_roll _relativerotation_pitch _relativerotation_yaw) (`KismetMathLibrary.BreakRotator` (`SceneComponent.RelativeRotation` (`self.Scene`))))
  (`SceneComponent.K2_SetRelativeLocation` (`self.Scene`) (`KismetMathLibrary.MakeVector` 23.0 (+ (/ _relativerotation_yaw 3.0) 20.0) 5.0) false false)
  (`SceneComponent.K2_SetRelativeRotation` :`self` (`self.Scene`)))

(event `/Game/Blueprints/Interfaces/BPI_Interaction.PlaySound`
  (params (Action :type String) (Actor :type "Actor Object Reference"))
  (bind _returnvalue (`self.K2_GetActorLocation` Actor))
  (bind _asbp_game_instance (cast `/Game/FirstPerson/Blueprints/BP_GameInstance` (`GameplayStatics.GetGameInstance`)))
  (bind _sfxvolume (`/Game/FirstPerson/Blueprints/BP_GameInstance.GetSfxVolume` _asbp_game_instance))
  (switch `string` Action
    (:`Open`
      (bind _returnvalue_2 (* _sfxvolume 5.0))
      (`GameplayStatics.PlaySoundAtLocation` "/Game/Audio/Sounds/DrawerOpening.DrawerOpening" _returnvalue (struct) _returnvalue_2 1.0 0.0 null null null null))
    (:`Close`
      (`KismetSystemLibrary.Delay` 0.2)
      (`GameplayStatics.PlaySoundAtLocation` "/Game/Audio/Sounds/DrawerClosing.DrawerClosing" _returnvalue (struct) _returnvalue_2 1.0 0.0 null null null null))))

(fn `Get State`
  (returns (isOpen :type Boolean))
  (return (`self.IsOpen`)))

(fn `UserConstructionScript`)