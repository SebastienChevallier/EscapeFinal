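; BP_Chessboard is a chessboard actor that slides along the Y axis when its MoveChessBoard event is called.
; The event clears the actor's tags, makes the MasterPiece component visible and plays a sliding sound at the root's location.
; A Timeline then drives the root's relative Y from an offset base, leaving X and Z unchanged.
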(event `MoveChessBoard`
  (bind _defaultsceneroot (`self.DefaultSceneRoot`))
  (bind (_relativelocation_x _relativelocation_y _relativelocation_z) (`KismetMathLibrary.BreakVector` (`SceneComponent.RelativeLocation` _defaultsceneroot)))
  (`KismetArrayLibrary.Array_Clear` (`self.Tags`))
  (`SceneComponent.SetVisibility` (`self.MasterPiece`) true false)
  (`GameplayStatics.PlaySoundAtLocation` "/Game/Audio/Sounds/SlidingLibrary.SlidingLibrary" (`SceneComponent.K2_GetComponentLocation` (`self.DefaultSceneRoot`)) (struct) 1.0 1.0 0.0 null null null null)
  (bind (_direction _movechessboard) (`Timeline|Timeline`)
    (:`Update`
      (`SceneComponent.K2_SetRelativeLocation` _defaultsceneroot (`KismetMathLibrary.MakeVector` _relativelocation_x (+ _movechessboard 136.0) _relativelocation_z) false false))))

(fn `UserConstructionScript`)