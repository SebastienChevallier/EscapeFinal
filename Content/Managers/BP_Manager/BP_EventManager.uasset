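; BP_EventManager is a manager actor that triggers the level's BP_Event actors by type or by elapsed game time.
; It caches all events on BeginPlay, then counts time on Tick and shows it as minutes:seconds on a TextRender.
; Timed events fire on every tick where their Time matches the minutes and total truncated seconds.
; TriggerEvent fires only the first event matching the requested enum type.
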(event `self.ReceiveBeginPlay`
  (bind _outactors (`GameplayStatics.GetAllActorsOfClass` "/Game/Events/Blueprint/BP_Event.BP_Event_C"))
  (set `self.EventList` _outactors)
  (set `self.GeneralTimer` 0.0))

(event `self.ReceiveTick`
  (params (DeltaSeconds :type "Float (single-precision)"))
  (bind _returnvalue (+ DeltaSeconds (`self.GeneralTimer`)))
  (bind _output_get (set `self.Secondes` (`KismetMathLibrary.FTrunc` _returnvalue)))
  (bind _output_get_2 (set `self.Minutes` (/ _output_get 60)))
  (set `self.GeneralTimer` _returnvalue)
  (`self.TriggerTimedEvent`)
  (`TextRenderComponent.K2_SetText` (`self.TextRender`) (`KismetTextLibrary.Conv_StringToText` (`KismetStringLibrary.Concat_StrStr` (`KismetStringLibrary.Conv_IntToString` (mod _output_get_2 60)) " : " (`KismetStringLibrary.Conv_IntToString` (mod _output_get 60)) " "))))

(fn `TriggerEvent`
  (params (EnumEvent :type "/Game/Managers/Enum_Event Enum" :default "NewEnumerator0"))
  (for _array_element (`self.EventList`)
    (if (`|EnumEquality` (`/Game/Events/Blueprint/BP_Event.EventType` _array_element) EnumEvent)
      (`/Game/Managers/BP_Interfaces/BPI_Event.TriggerEvent` _array_element)
      (break))))

(fn `TriggerTimedEvent`
  (for _array_element (`self.EventList`)
    (if (`/Game/Events/Blueprint/BP_Event.TimedEvent` _array_element)
      (bind (_x _y) (`KismetMathLibrary.BreakVector2D` (`/Game/Events/Blueprint/BP_Event.Time` _array_element)))
      (if (and (== _x (`self.Minutes`)) (== _y (`self.Secondes`)))
        (`/Game/Managers/BP_Interfaces/BPI_Event.TriggerEvent` _array_element)))))

(fn `UserConstructionScript`)