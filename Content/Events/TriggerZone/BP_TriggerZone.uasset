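; BP_TriggerZone is a trigger volume that fires game events when the first-person character enters or leaves it.
; On BeginPlay it finds and caches the BP_EventManager in the level.
; Begin and end overlaps loop over the EventsToTrigger array, using each entry's EnterOrExit flag to pick enter or exit events.
; Matching entries pass their event enum to the manager's TriggerEvent.
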(event `self.ReceiveBeginPlay`
  (bind _returnvalue (`GameplayStatics.GetActorOfClass` "/Game/Managers/BP_Manager/BP_EventManager.BP_EventManager_C"))
  (set `self.EventManager` _returnvalue))

(event `self.TriggerZone.OnComponentBeginOverlap`
  (params (OverlappedComponent :type "PrimitiveComponent Object Reference") (OtherActor :type "Actor Object Reference") (OtherComp :type "PrimitiveComponent Object Reference") (OtherBodyIndex :type Integer) (bFromSweep :type Boolean) (SweepResult :type "HitResult Structure (by ref)"))
  (cast `/Game/FirstPerson/Blueprints/BP_FirstPersonCharacter` OtherActor)
  (for _array_element (`self.EventsToTrigger`)
    (bind (_eventenum _enterorexit) (break `/Game/Events/Blueprint/EventType` _array_element))
    (if _enterorexit
      (`self.CallEventTrigger` _eventenum))))

(event `self.TriggerZone.OnComponentEndOverlap`
  (params (OverlappedComponent :type "PrimitiveComponent Object Reference") (OtherActor :type "Actor Object Reference") (OtherComp :type "PrimitiveComponent Object Reference") (OtherBodyIndex :type Integer))
  (cast `/Game/FirstPerson/Blueprints/BP_FirstPersonCharacter` OtherActor)
  (for _array_element (`self.EventsToTrigger`)
    (bind (_eventenum _enterorexit) (break `/Game/Events/Blueprint/EventType` _array_element))
    (if (not _enterorexit)
      (`self.CallEventTrigger` _eventenum))))

(fn `CallEventTrigger`
  (params (EventEnum :type "/Game/Managers/Enum_Event Enum" :default "NewEnumerator0"))
  (`/Game/Managers/BP_Manager/BP_EventManager.TriggerEvent` (`self.EventManager`) EventEnum))

(fn `UserConstructionScript`)