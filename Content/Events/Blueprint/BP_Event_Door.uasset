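; BP_Event_Door is a triggered event actor that advances a door through three staged sequences.
; Each TriggerEvent call plays the next of three ActorSequence components, tracked by a Step counter.
; After the third sequence plays, IsPlayed is set so further triggers do nothing.
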(event `/Game/Managers/BP_Interfaces/BPI_Event.TriggerEvent`
  (if (not (`self.isPlayed`))
    (switch `int` (`self.Step`)
      (:`0`
        (`ActorSequenceComponent.PlaySequence` (`self.ActorSequence`))
        (set `self.Step` 1))
      (:`1`
        (`ActorSequenceComponent.PlaySequence` (`self.ActorSequence1`))
        (set `self.Step` 2))
      (:`2`
        (`ActorSequenceComponent.PlaySequence` (`self.ActorSequence2`))
        (set `self.isPlayed` true)))))

(fn `UserConstructionScript`
  (`parent.UserConstructionScript`))