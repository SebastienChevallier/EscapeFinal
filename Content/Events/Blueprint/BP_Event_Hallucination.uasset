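; Hallucination event actor that, once triggered, gradually distorts the view through the level's post-process volume and activates smoke.
; TriggerEvent puts MaterialInstance in the volume's first post-process material slot and enables a Tick blend.
; Tick slowly ramps post-process intensity, drives the material's Speed with a growing sine of game time, and re-activates Smoke.
; The dynamic material creation nodes are disconnected and never run.
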(event `self.ReceiveBeginPlay`
  (`ActorComponent.Activate` (`self.Smoke`) false)
  (bind _returnvalue (`GameplayStatics.GetActorOfClass` "/Script/Engine.PostProcessVolume"))
  (set `self.PostProcessVolume` _returnvalue))

(event `/Game/Managers/BP_Interfaces/BPI_Event.TriggerEvent`
  (set `self.canLerp` true)
  (setmembers `WeightedBlendable` :`StructRef` (`|GetArrayItem` (`.Array` (break `WeightedBlendables` (`.WeightedBlendables` (break `PostProcessSettings` (`PostProcessVolume.Settings` (`self.PostProcessVolume`))))))) :`Object` (`self.materialInstance`)))

(event `self.ReceiveTick`
  (params (DeltaSeconds :type "Float (single-precision)"))
  (bind _returnvalue (`KismetMathLibrary.FClamp` (+ (* DeltaSeconds 0.01) (`self.PowerMultiply`))))
  (if (`self.canLerp`)
    (set `self.PowerMultiply` _returnvalue)
    (setmembers `PostProcessSettings` :`StructRef` (`PostProcessVolume.Settings` (`self.PostProcessVolume`)) :`SceneFringeIntensity` (`KismetMathLibrary.Lerp` 0.0 1.0 _returnvalue))
    (`MaterialInstanceDynamic.SetScalarParameterValue` (`self.materialInstance`) "Speed" (`KismetMathLibrary.Lerp` 0.0 2.0 (* (* _returnvalue (`KismetMathLibrary.Sin` (`self.GetGameTimeSinceCreation`))) 1.0)))
    (`ActorComponent.Activate` (`self.Smoke`) false)))

(fn `UserConstructionScript`
  (`parent.UserConstructionScript`))