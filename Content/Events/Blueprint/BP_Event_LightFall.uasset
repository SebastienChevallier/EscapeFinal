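; Scripted event actor that drops a light bulb once when triggered.
; TriggerEvent enables gravity on the bulb and activates the Electric effect, with an IsPlayed flag blocking repeats.
; When the bulb's hit event reports contact with the Ground component, the point light's intensity drops to zero and the audio, stopped at BeginPlay, plays.
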(event `self.ReceiveBeginPlay`
  (`AudioComponent.Stop` (`self.Audio`)))

(event `self.LightBulb.OnComponentHit`
  (params (HitComponent :type "PrimitiveComponent Object Reference") (OtherActor :type "Actor Object Reference") (OtherComp :type "PrimitiveComponent Object Reference") (NormalImpulse :type "Vector Structure") (Hit :type "HitResult Structure (by ref)"))
  (if (== (`self.Ground`) OtherComp)
    (`LightComponent.SetIntensity` (`self.PointLight`) 0.0)
    (`AudioComponent.Play` (`self.Audio`) 0.0)))

(event `/Game/Managers/BP_Interfaces/BPI_Event.TriggerEvent`
  (if (not (`self.isPlayed`))
    (`PrimitiveComponent.SetEnableGravity` (`self.LightBulb`) true)
    (`ActorComponent.Activate` (`self.Electric`) true)
    (set `self.isPlayed` true)))

(fn `UserConstructionScript`
  (`parent.UserConstructionScript`))