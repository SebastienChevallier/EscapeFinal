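; Event Blueprint for a spot light flicker that runs over a set duration.
; Tick accumulates time up to FlickDuration and sets a randomized sine of game time scaled by the intensity cached at BeginPlay.
; As wired, the same tick then overwrites that value with zero or the cached intensity, depending on LightOffAfterFlick.
; TriggerEvent sets a Flick flag that Tick never reads.
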(event `self.ReceiveBeginPlay`
  (set `self.lightIntensity` (`LightComponentBase.Intensity` (`self.SpotLight`))))

(event `self.ReceiveTick`
  (params (DeltaSeconds :type "Float (single-precision)"))
  (bind _actualduration (`self.actualDuration`))
  (if (<= _actualduration (`self.FlickDuration`))
    (set `self.actualDuration` (+ _actualduration DeltaSeconds))
    (`LightComponent.SetIntensity` (`self.SpotLight`) (* (`KismetMathLibrary.Sin` (* (`GameplayStatics.GetTimeSeconds`) 2.0 (`KismetMathLibrary.RandomFloatInRange` 0.0 (`self.FlickPower`)))) (`self.lightIntensity`)))
    (if (`self.LightOffAfterFlick`)
      (`LightComponent.SetIntensity` (`self.SpotLight`) 0.0)
      (else
        (`LightComponent.SetIntensity` (`self.SpotLight`) (`self.lightIntensity`))))))

(event `/Game/Managers/BP_Interfaces/BPI_Event.TriggerEvent`
  (set `self.bFlick` true))

(fn `UserConstructionScript`
  (`parent.UserConstructionScript`))