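; BP_Enigme is a puzzle controller that counts completed tasks and reveals a picture when the puzzle ends.
; CompleteTask increments ProgressionIndex and calls EndEnigme once it reaches the TaskList length, making Picture and its child components visible.
; It ignores which task was passed in: the logic for starting tasks and gating their order is disconnected.
; TryCompletetask is an empty stub.
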(event `self.ReceiveBeginPlay`)

(fn `CompleteTask`
  (params (CurrentTask :type "/Game/Enigmes/BP_Task Object Reference") (Player :type "/Game/FirstPerson/Blueprints/BP_FirstPersonCharacter Object Reference"))
  (bind _result (`/Engine/EditorBlueprintResources/StandardMacros.IncrementInt` (`self.ProgressionIndex`))
    (:`  `
      (if (>= _result (`KismetArrayLibrary.Array_Length` (`self.TaskList`)))
        (`self.EndEnigme`)))))

(fn `EndEnigme`
  (`SceneComponent.SetVisibility` (`Actor.RootComponent` (`self.Picture`)) true true))

(fn `TryCompletetask`
  (params (Task :type "/Game/Enigmes/BP_Task Object Reference")))

(fn `UserConstructionScript`)