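; BP_TouchBlockTask is a debug puzzle task that completes when the first-person character touches its sphere.
; It calls OnStart on BeginPlay, which runs the parent logic and shows the sphere only if CanComplete is true.
; An overlap by the character calls OnComplete without rechecking CanComplete, running the parent completion logic and hiding the sphere.
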(event `self.Sphere.OnComponentBeginOverlap`
  (params (OverlappedComponent :type "PrimitiveComponent Object Reference") (OtherActor :type "Actor Object Reference") (OtherComp :type "PrimitiveComponent Object Reference") (OtherBodyIndex :type Integer) (bFromSweep :type Boolean) (SweepResult :type "HitResult Structure (by ref)"))
  (cast `/Game/FirstPerson/Blueprints/BP_FirstPersonCharacter` OtherActor)
  (`self.OnComplete`))

(event `self.ReceiveBeginPlay`
  (`self.OnStart`))

(fn `OnComplete`
  (`parent.OnComplete`)
  (`SceneComponent.SetVisibility` (`self.Sphere`) false false))

(fn `OnStart`
  (`parent.OnStart`)
  (if (`self.CanComplete`)
    (`SceneComponent.SetVisibility` (`self.Sphere`) true false)
    (else
      (`SceneComponent.SetVisibility` (`self.Sphere`) false false))))

(fn `UserConstructionScript`
  (`parent.UserConstructionScript`))