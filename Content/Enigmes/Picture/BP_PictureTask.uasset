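; BP_PictureTask is a pickup task actor for the picture puzzle, built on a parent class that supplies pickup and completion behavior.
; It hides its root and all child components at BeginPlay.
; Pickup runs the parent logic, then sets its PictureIndex entry in the BPPictureEnime PicturePickup array to false.
; Drop is empty with no parent call, and completion runs the parent logic before destroying the actor.
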(event `self.ReceiveBeginPlay`
  (`SceneComponent.SetVisibility` (`self.DefaultSceneRoot`) false true))

(fn `Drop`)

(fn `OnComplete`
  (`parent.OnComplete`)
  (`self.K2_DestroyActor`))

(fn `Pickup`
  (`parent.Pickup`)
  (`KismetArrayLibrary.Array_Set` (`/Game/Enigmes/Picture/BP_PictureEnigme.PicturePickup` (`self.BP_PictureEnime`)) (`self.PictureIndex`)))

(fn `UserConstructionScript`
  (`parent.UserConstructionScript`))